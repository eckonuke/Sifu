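; Enemy character Blueprint that pursues the player and can be offered up as a finisher target.
; Each Tick it moves straight toward the first player character with movement input, without pathfinding, only while farther than a set standoff distance.
; While the enemy is not dead, actors that begin overlapping its Box component receive SetFinishableMessage with the enemy as argument, which supports the special finishing move.
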(event `self.ReceiveTick`
  (params (DeltaSeconds :type "Float (single-precision)"))
  (bind _returnvalue (`GameplayStatics.GetPlayerCharacter` 0))
  ;[1 1 1] 적이 플레이어 한테 다가갈수 있도록(일정 거리를 둔다)
  (`parent.ReceiveTick` DeltaSeconds)
  (`/Engine/EditorBlueprintResources/StandardMacros.IsValid` _returnvalue
    (:`Is Valid`
      (if (> (`self.GetDistanceTo` _returnvalue self) 400.0)
        (`self.AddMovementInput` (`KismetMathLibrary.GetDirectionUnitVector` (`self.K2_GetActorLocation` self) (`self.K2_GetActorLocation` _returnvalue)))))))

(event `self.Box.OnComponentBeginOverlap`
  (params (OverlappedComponent :type "PrimitiveComponent Object Reference") (OtherActor :type "Actor Object Reference") (OtherComp :type "PrimitiveComponent Object Reference") (OtherBodyIndex :type Integer) (bFromSweep :type Boolean) (SweepResult :type "HitResult Structure (by ref)"))
  ;[1 1 1] 필살기 실행
  (if (not (`self.dead`))
    (message `/Game/Blueprint/BPI_Finisher.SetFinishable` OtherActor self)))

(fn `UserConstructionScript`
  (`parent.UserConstructionScript`))