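; Game mode that creates the player's HUD and keeps its health values current.
; On BeginPlay it caches player 0's character as Player_KYI, then creates the player UI widget and adds it to the viewport; a failed cast skips the UI setup.
; Every Tick, UpdateHealth pushes the character's current and max HP into the widget by polling, with no validity check on either reference.
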(event `self.ReceiveBeginPlay`
  (bind _asplayer_kyi (cast `Player_KYI` (`GameplayStatics.GetPlayerCharacter` 0)))
  (set `self.player` _asplayer_kyi)
  (bind _returnvalue (`|CreateWidget` "/Game/SideScrollerBP/UI/PlayerUI.PlayerUI_C" (`GameplayStatics.GetPlayerController` 0)))
  (bind _output_get (set `self.playerUI` _returnvalue))
  (`UserWidget.AddToViewport` _output_get 0))

(event `self.ReceiveTick`
  (params (DeltaSeconds :type "Float (single-precision)"))
  (`self.updateHealth`))

(fn `updateHealth`
  (bind _player (`self.player`))
  (bind _playerui (`self.playerUI`))
  (set `/Game/SideScrollerBP/UI/PlayerUI.currentHP` (`Player_KYI.currHp` _player) _playerui)
  (set `/Game/SideScrollerBP/UI/PlayerUI.maxHP` (`Player_KYI.maxHp` _player) _playerui))

(fn `UserConstructionScript`)